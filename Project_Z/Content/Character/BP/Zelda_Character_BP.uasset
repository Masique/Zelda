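; Player character Blueprint for Zelda that handles movement, look, crouch and torch-lighting input.
; Axis inputs drive controller yaw and pitch and move along the actor's forward and right vectors, while crouch lasts as long as its input is held.
; Lighting the torch stops and disables movement, sets IsLighting, then restores walking after a short delay; the flag is never cleared here.
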(event `InputAxis|Rotate_Left_Right`
  (params (AxisValue :type "Float (single-precision)"))
  ;[1 1 1] rotate_left_right_Look_up_down
  (`self.AddControllerYawInput` AxisValue))

(event `InputAxis|Forward_Backward`
  (params (AxisValue :type "Float (single-precision)"))
  ;[1 1 1] Move_forward_backward_left_right
  (`self.AddMovementInput` (`self.GetActorForwardVector`) AxisValue))

(event `InputAxis|Look_up_down`
  (params (AxisValue :type "Float (single-precision)"))
  ;[1 1 1] rotate_left_right_Look_up_down
  (`self.AddControllerPitchInput` AxisValue))

(event `InputAxis|Strafe_Left_Right`
  (params (AxisValue :type "Float (single-precision)"))
  ;[1 1 1] Move_forward_backward_left_right
  (`self.AddMovementInput` (`self.GetActorRightVector`) AxisValue))

(event `InputAction|Crouch`
  (params (Key :type "Key Structure"))
  ;[1 1 1] crouch
  (:`Pressed`
    (`self.Crouch`))
  (:`Released`
    (`self.UnCrouch`)))

(event `InputAction|Light_torch`
  (params (Key :type "Key Structure"))
  ;[1 1 1] Light_Torch
  (:`Pressed`
    (`CharacterMovementComponent.DisableMovement` (`self.CharacterMovement`))
    (`MovementComponent.StopMovementImmediately` (`self.CharacterMovement`))
    (set `self.IsLighting?` true)
    (`KismetSystemLibrary.Delay` 0.2)
    (`CharacterMovementComponent.SetMovementMode` (`self.CharacterMovement`) "MOVE_Walking" 0)))

(fn `UserConstructionScript`)